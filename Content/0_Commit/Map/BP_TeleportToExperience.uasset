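; BP_TeleportToExperience is a map trigger actor that sends the local player into another experience when their pawn overlaps its Cube.
; The overlap handler filters for a pawn with a local player controller and passes that controller to LoadIntoExperience.
; That event creates a hosting request from the assigned UserFacingExperience, sets it to offline mode, and hosts the session through CommonSessionSubsystem.
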(event OnComponentBeginOverlap(Cube)
  (params (OverlappedComponent :type Primitive%20Component%20Object%20Reference) (OtherActor :type Actor%20Object%20Reference) (OtherComp :type Primitive%20Component%20Object%20Reference) (OtherBodyIndex :type Integer) (bFromSweep :type Boolean) (SweepResult :type Hit%20Result%20Structure%20%28by%20ref%29))
  (Development|PrintString "Overlap!")
  (bind _aspawn (Utilities|Casting|CastToPawn OtherActor))
  (Utilities|IsValid (Pawn|GetController _aspawn)
    (:Is%20Valid
      (if (Pawn|IsLocalPlayerController (Pawn|GetController _aspawn))
        (bind _asplayer_controller (Utilities|Casting|CastToPlayerController (Pawn|GetController _aspawn)))
        (CallFunction|LoadIntoExperience _asplayer_controller)))))

(event Custom|Load%20Into%20Experience
  (params (NewParam :type Player%20Controller%20Object%20Reference))
  (bind _userfacingexperience (Variables|Default|GetUserFacingExperience))
  (Utilities|IsValid _userfacingexperience
    (:Is%20Valid
      (bind _returnvalue (Class|DestinyUserFacingExperience|CreateHostingRequest _userfacingexperience))
      (Variables|/Script/CommonUser.CommonSession_HostSessionRequest|SetOnlineMode _returnvalue "Offline")
      (Class|CommonSessionSubsystem|HostSession (Subsystems|GetCommonSessionSubsystem) NewParam 0))))

(event EventBeginPlay)

(event Collision|EventActorBeginOverlap
  (params (OtherActor :type Actor%20Object%20Reference)))

(event EventTick
  (params (DeltaSeconds :type Float%20%28single-precision%29)))

(fn ConstructionScript)